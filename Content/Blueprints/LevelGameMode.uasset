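; Game mode that runs a last-player-standing round loop for Revenant player characters.
; It collects player controllers at login, and PlayerKilled decrements and prints the alive count, triggering RestartLevel at one or fewer.
; RestartLevel revives each player's pawn in place of reloading the map, moving it to a random, possibly shared PlayerStart.
; It resets PlayersAlive to zero, and nothing in this graph increments that count.
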(event Custom|RestartLevel
  (Variables|Default|SetplayersAlive 0)
  (for _array_element (Variables|Default|GetPlayerControllers)
    (bind _outactors (Actor|GetAllActorsOfClass "/Script/Engine.PlayerStart"))
    (bind _asrevenant_player_character (Utilities|Casting|CastToRevenantPlayerCharacter (Pawn|GetControlledPawn _array_element)))
    (Default|Revive _asrevenant_player_character)
    (Transformation|SetActorTransform _asrevenant_player_character (Transformation|GetActorTransform (Utilities|Array|Get(acopy) _outactors (Math|Random|RandomIntegerinRange 0 (- (Utilities|Array|Length _outactors) 1)))))))

(event EventPostLogin
  (params (NewPlayer :type Player%20Controller%20Object%20Reference))
  (Utilities|Array|Add (Variables|Default|GetPlayerControllers) NewPlayer))

(fn ConstructionScript)

(fn PlayerKilled
  (bind _result (Math|Integer|DecrementInt (Variables|Default|GetplayersAlive))
    (:%20%20
      (Development|PrintString (Utilities|String|ToString(Integer) _result))
      (if (<= _result 1)
        (CallFunction|RestartLevel)))))