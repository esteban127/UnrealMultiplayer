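; Behavior tree task that puts an Enemy into patrol mode and picks its next patrol destination.
; It applies the patrol speed, clears the Chasing flag and writes a random reachable point within PatrolRadius to the PatrolLocation blackboard key.
; If no point is found, it stores the pawn's current location instead.
; The task fails only when the controlled pawn is not an Enemy.
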(event EventReceiveExecuteAI
  (params (OwnerController :type AI%20Controller%20Object%20Reference) (ControlledPawn :type Pawn%20Object%20Reference))
  (bind _returnvalue (Transformation|GetActorLocation ControlledPawn))
  (bind _patrollocation (Variables|Default|GetPatrolLocation))
  (bind _patrolradius (Variables|Default|GetPatrolRadius))
  (bind (_randomlocation _returnvalue_2) (AI|Navigation|GetRandomReachablePointinRadius _returnvalue _patrolradius 0 0))
  (bind _asenemy (Utilities|Casting|CastToEnemy ControlledPawn)
    (:then
      (Default|UpdateSpeed _asenemy (Variables|Default|GetPatrolSpeed))
      (Variables|/Game/Blueprints/Enemy.Enemy_C|Setchasing _asenemy false)
      (if _returnvalue_2
        (AI|BehaviorTree|SetBlackboardValueasVector _patrollocation _randomlocation)
        (else
          (AI|BehaviorTree|SetBlackboardValueasVector _patrollocation _returnvalue)))
      (AI|BehaviorTree|FinishExecute true))
    (:CastFailed
      (AI|BehaviorTree|FinishExecute false))))