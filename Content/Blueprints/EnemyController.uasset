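; EnemyController is an enemy AI controller that runs a behavior tree on possess and tracks the player through AI perception.
; A successful sense of a Player-tagged actor cancels the loss timer and writes line of sight and the actor to the Blackboard.
; Any other perception update starts a timer that clears both keys on expiry, giving the enemy a grace period before losing its target.
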(event OnTargetPerceptionUpdated(AIPerception)
  (params (Actor :type Actor%20Object%20Reference) (Stimulus :type AI%20Stimulus%20Structure))
  (if (and (Actor|ActorHasTag Actor "Player") (.bSuccessfullySensed (Utilities|Struct|BreakAIStimulus Stimulus)))
    (Utilities|Time|ClearandInvalidateTimerbyHandle (Variables|Default|GetTimeHandler))
    (bind _blackboardcomponent (Class|AIController|UseBlackboard "/Game/Blueprints/BlackboardData.BlackboardData"))
    (AI|Components|Blackboard|SetValueasBool _blackboardcomponent (Variables|Default|GetLineOfSight) true)
    (AI|Components|Blackboard|SetValueasObject _blackboardcomponent (Variables|Default|GetEnemyActor) Actor)
    (else
      (bind _returnvalue (Utilities|Time|SetTimerbyEvent (delegate Custom|StartEnemyTimer) (Variables|Default|GetLineOfSightTimer)))
      (Variables|Default|SetTimeHandler _returnvalue))))

(event Custom|StartEnemyTimer
  (bind _blackboardcomponent (Class|AIController|UseBlackboard "/Game/Blueprints/BlackboardData.BlackboardData"))
  (AI|Components|Blackboard|SetValueasBool _blackboardcomponent (Variables|Default|GetLineOfSight) false)
  (AI|Components|Blackboard|SetValueasObject _blackboardcomponent (Variables|Default|GetEnemyActor) 0))

(event EventPossess
  (params (PossessedPawn :type Pawn%20Object%20Reference))
  (AI|RunBehaviorTree "/Game/Blueprints/BehaviorTree.BehaviorTree"))

(fn ConstructionScript)